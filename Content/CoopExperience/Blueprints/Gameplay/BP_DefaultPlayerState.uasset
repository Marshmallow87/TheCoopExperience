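; Co-op player state that tracks the player's health and requests a respawn on death.
; On BeginPlay the server caches the owning PlayerController.
; AnyDamage received by the player state subtracts from current health and prints it.
; At zero or below, the server asks BP_DefaultGameMode to respawn that controller with the stored HeroCharacter class.
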(event EventBeginPlay
  (bind _returnvalue (Components|GetOwner))
  ;[1 1 1] Sets A Reference to the PlayerController
  (Networking|SwitchHasAuthority
    (:Authority
      (Utilities|IsValid _returnvalue
        (:Is%20Valid
          (bind _asplayer_controller (Utilities|Casting|CastToPlayerController _returnvalue)
            (:then
              (Variables|Default|SetMyPlayerController _asplayer_controller))
            (:CastFailed
              (Development|PrintString "Cast TO PlayerController Failed"))))))))

(event Game|Damage|EventAnyDamage
  (params (Damage :type Float%20%28single-precision%29) (DamageType :type Damage%20Type%20Object%20Reference) (InstigatedBy :type Controller%20Object%20Reference) (DamageCauser :type Actor%20Object%20Reference))
  (bind _output_get (Variables|Default|SetCurrentHealth (- (Variables|Default|GetCurrentHealth) Damage)))
  (Development|PrintString (Utilities|String|ToString(Float) _output_get))
  (if (<= _output_get 0.0) ; Is Dead?
    ;[1 1 1] If Player Dies
    (Networking|SwitchHasAuthority
      (:Authority
        (bind _asbp_default_game_mode (Utilities|Casting|CastToBP_DefaultGameMode (Game|GetGameMode))
          (:then
            (Class|DefaultGameMode|RespawnPlayer _asbp_default_game_mode "/Game/HeroCharacter.HeroCharacter_C" (Variables|Default|GetMyPlayerController)))
          (:CastFailed
            (Development|PrintString "Cast To BP_MainGameMode Failed")))))))

(fn ConstructionScript)