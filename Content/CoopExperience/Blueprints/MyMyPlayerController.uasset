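; Player controller for the CoopExperience game that sets up the health bar UI and provides a test input for self-inflicted damage.
; On BeginPlay it creates a BP_HealthBar widget owned by itself and adds it to the viewport.
; The TEST_TakeDamage action calls an SRV-prefixed event with a fixed amount, applying damage to the PlayerState rather than the pawn.
; A separate TakeDamage event duplicates that ApplyDamage call.
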(event Custom|SRV_TakeDamage
  (params (Damage :type Float%20%28single-precision%29))
  (Game|Damage|ApplyDamage (Variables|Default|GetPlayerState) Damage 0 0))

(event Custom|TakeDamage
  (params (Damage :type Float%20%28single-precision%29))
  (Game|Damage|ApplyDamage (Variables|Default|GetPlayerState) Damage 0 0))

(event Custom|AddHealthBarWidget
  (Development|PrintString "Ivyko AddHealthBarWidget")
  (bind _returnvalue (UserInterface|CreateWidget "/Game/CoopExperience/HUD/BP_HealthBar.BP_HealthBar_C" self))
  (UserInterface|Viewport|AddtoViewport _returnvalue 0))

(event EventBeginPlay
  (CallFunction|AddHealthBarWidget))

(event EventTick
  (params (DeltaSeconds :type Float%20%28single-precision%29)))

(event Input|ActionEvents|InputActionTEST_TakeDamage
  (params (Key :type Key%20Structure :default "None"))
  (:Pressed
    (Development|PrintString "L Pressed")
    (CallFunction|SRVTakeDamage 36.0)))

(fn ConstructionScript)