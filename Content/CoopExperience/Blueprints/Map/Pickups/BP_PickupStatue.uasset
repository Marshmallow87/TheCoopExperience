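; BP_PickupStatue is an interactable map pickup that grants gold to the player who collects it.
; Interact runs only with authority and passes the instigator to the Pickup event.
; Pickup casts the instigator to the first-person character, adds a fixed gold amount to its player state, spawns an explosion effect with a sound, and destroys the actor.
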(event Custom|Pickup
  (params (Instigator :type Actor%20Object%20Reference))
  (bind _asbp_first_person_character (Utilities|Casting|CastToBP_FirstPersonCharacter Instigator))
  (bind _asbp_default_player_state (Utilities|Casting|CastToBP_DefaultPlayerState (Variables|/Script/Engine.Pawn|GetPlayerState _asbp_first_person_character)))
  (Variables|/Script/TheCoopExperience.DefaultPlayerState|SetGold _asbp_default_player_state (+ (Variables|/Script/TheCoopExperience.DefaultPlayerState|GetGold _asbp_default_player_state) 50))
  (Effects|SpawnEmitteratLocation "/Game/StarterContent/Particles/P_Explosion.P_Explosion" (Transformation|GetActorLocation))
  (Audio|PlaySoundatLocation "/Game/CoopExperience/Sounds/pickup_item_sound_Cue.pickup_item_sound_Cue" (Transformation|GetActorLocation) "0, 0, 0" 1.0 1.0 0.0 0 0 0)
  (Actor|DestroyActor))

(fn ConstructionScript)

(fn Interact
  (params (Actor :type Actor%20Object%20Reference) (ActorComponent :type Actor%20Component%20Object%20Reference) (Instigator :type Actor%20Object%20Reference))
  (Networking|SwitchHasAuthority
    (:Authority
      (CallFunction|Pickup Instigator)
      (return false))))