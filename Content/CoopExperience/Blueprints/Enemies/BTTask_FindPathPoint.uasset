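; Behavior tree task that gives a BP_Enemy its next patrol destination from its assigned PatrolPath.
; It reads the path index from the blackboard, converts that path point from the path actor's local space to world space and writes it to the vector key.
; It finishes successfully after a short delay, but never calls FinishExecute when the cast fails or the path is invalid.
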(event EventReceiveExecuteAI
  (params (OwnerController :type AI%20Controller%20Object%20Reference) (ControlledPawn :type Pawn%20Object%20Reference))
  (bind _asbp_enemy (Utilities|Casting|CastToBP_Enemy ControlledPawn)
    (:then
      (bind _patrolpath (Variables|/Game/CoopExperience/Blueprints/Enemies/BP_Enemy.BP_Enemy_C|GetPatrolPath _asbp_enemy)
        (:then
          (bind _output_get (Variables|Default|SetBB_PathVector (Variables|Default|GetBB_PathVector)))
          (AI|BehaviorTree|SetBlackboardValueasVector _output_get (Math|Transform|TransformLocation (Transformation|GetActorTransform _patrolpath) (Utilities|Array|Get(acopy) (Variables|/Game/CoopExperience/Blueprints/Enemies/PatrolPath.PatrolPath_C|GetPathPoints _patrolpath) (Class|BTFunctionLibrary|GetBlackboardValueasInt (Variables|Default|GetBB_PathIndex)))))
          (Utilities|FlowControl|Delay 1.0)
          (AI|BehaviorTree|FinishExecute true))
        (:else)))
    (:CastFailed
      (Development|PrintString "cast"))))