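; Behavior tree task that snaps a BP_Enemy to face the player it perceives.
; It computes a look-at rotation from the AI controller's location to PerceivedPlayer and applies it as the control rotation.
; The enemy actor takes that yaw with a -90 degree offset, then the task finishes successfully.
; Both validity branches continue identically, and a failed cast never finishes the task.
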(event EventReceiveExecuteAI
  (params (OwnerController :type AI%20Controller%20Object%20Reference) (ControlledPawn :type Pawn%20Object%20Reference))
  (bind _asbp_enemy (Utilities|Casting|CastToBP_Enemy ControlledPawn))
  (bind _perceivedplayer (Variables|/Game/CoopExperience/Blueprints/Enemies/BP_Enemy.BP_Enemy_C|GetPerceivedPlayer _asbp_enemy)
    (:then
      _)
    (:else
      _))
  (Pawn|SetControlRotation OwnerController (Math|Rotator|FindLookatRotation (Transformation|GetActorLocation OwnerController) (Transformation|GetActorLocation _perceivedplayer)))
  (bind _asbp_enemy_2 (Utilities|Casting|CastToBP_Enemy ControlledPawn))
  (Transformation|SetActorRotation _asbp_enemy_2 (Math|Rotator|MakeRotator 0.0 0.0 (+ (.Yaw (Math|Rotator|BreakRotator (Math|Rotator|FindLookatRotation (Transformation|GetActorLocation OwnerController) (Transformation|GetActorLocation _perceivedplayer)))) -9e+01)))
  (AI|BehaviorTree|FinishExecute true))