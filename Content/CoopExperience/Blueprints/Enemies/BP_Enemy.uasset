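; BP_Enemy is an enemy that shoots a first-person weapon Blueprint held in its Gun child actor.
; The Fire event casts that child to BP_FirstPersonWeapon and calls SRVFireWeapon with an origin raised above the mesh location and the control rotation as aim.
; It then plays a quiet pistol sound at the enemy's location.
; BeginPlay, Tick and the construction script are empty, so nothing in this Blueprint triggers Fire.
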(event Custom|Fire
  (bind _returnvalue (Pawn|GetControlRotation :!class /Script/Engine.Pawn))
  (bind _mesh (Variables|Character|GetMesh))
  (bind _returnvalue_2 (Transformation|GetWorldLocation _mesh))
  (bind _asbp_first_person_weapon (Utilities|Casting|CastToBP_FirstPersonWeapon (Variables|/Script/Engine.ChildActorComponent|GetChildActor (Variables|Default|GetGun))))
  (Default|SRVFireWeapon _asbp_first_person_weapon (Math|Vector|MakeVector (.x _returnvalue_2) (.y _returnvalue_2) (+ (.z _returnvalue_2) 1.5e+02)) (Math|Rotator|MakeRotator (.roll _returnvalue) (.pitch _returnvalue) (.yaw _returnvalue)))
  (Audio|PlaySoundatLocation "/Game/CoopExperience/Sounds/Pistol_shoot_sound_Cue.Pistol_shoot_sound_Cue" (Transformation|GetActorLocation) "0, 0, 0" 0.1 1.0 0.0 0 0 0))

(event EventBeginPlay)

(event EventTick
  (params (DeltaSeconds :type Float%20%28single-precision%29)))

(fn ConstructionScript)