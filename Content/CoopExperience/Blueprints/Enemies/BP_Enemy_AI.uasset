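; AI controller for enemies in the co-op game that starts the BT_Enemy behavior tree on BeginPlay.
; Enemy decision-making is left to that tree, as the controller has no other active logic.
; An unconnected perception fragment, which never runs, would store the detected first-person player and set the CanSeePlayer blackboard key to false for Player-tagged actors.
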(event EventBeginPlay
  (AI|RunBehaviorTree "/Game/CoopExperience/Blueprints/Enemies/BT_Enemy.BT_Enemy"))

(fn ConstructionScript)